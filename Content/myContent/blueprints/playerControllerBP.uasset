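; Player controller that drives an RTS camera pawn, cached on BeginPlay along with its start transform and spring arm length for later resets.
; Axis input moves the pawn relative to its facing at locked start height, with a speed modifier.
; Zoom inputs adjust the clamped arm length.
; Holding pan opens gates feeding mouse motion into yaw and clamped pitch, suspending the macro-based screen-edge scrolling that otherwise offsets the pawn.
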(event `self.ReceiveBeginPlay`
  ;[1 1 1] Reference casting and wakeup call
  (`|ExecutionSequence`
    (:`then_0`
      (`self.referenceCast`) ; This is going to control the camera via references
    )
    (:`then_1`
      (set `self.levelStart` (`self.GetTransform` (`self.cameraPawnRef`))) ; Automatically sets the future return point to the level designers start point
      (set `self.springArmLengthDefault` (`SpringArmComponent.TargetArmLength` (`/Game/myContent/blueprints/rtsCameraPawnBP.SpringArm` (`self.cameraPawnRef`)))) ; Get's the rigging default length and apply that to the game's default length
    )
    (:`then_2`
      (set `self.disableCameraMovement` false) ; Last thing to do is to unlock the camera
    )))

(event `InputAxis|inpMoveForward`
  (params (AxisValue :type "Float (single-precision)"))
  ;[1 1 1] X Y movement
  (`self.basicMovementControls` AxisValue (stale `InputAxis|inpMoveRight` AxisValue) :!label _label))

(event `InputAxis|inpMoveRight`
  (params (AxisValue :type "Float (single-precision)"))
  ;[1 1 1] X Y movement
  (goto _label))

(event `InputAction|inpSpeedModifier`
  (params (Key :type "Key Structure"))
  (bind _movemodifier (`self.moveModifier`))
  (bind _movespeedmultiuplier (`self.moveSpeedMultiuplier`))
  ;[1 1 1] X Y movement
  (:`Pressed`
    (set `self.moveModifier` (* _movemodifier _movespeedmultiuplier)))
  (:`Released`
    (set `self.moveModifier` (/ _movemodifier _movespeedmultiuplier))))

(event `InputAction|inpZoomReset`
  (params (Key :type "Key Structure"))
  ;[1 1 1] Reset Zoom
  (:`Released`
    (set `SpringArmComponent.TargetArmLength` (`self.springArmLengthDefault`) (`/Game/myContent/blueprints/rtsCameraPawnBP.SpringArm` (`self.cameraPawnRef`)))))

(event `InputAction|inpZoomIn`
  (params (Key :type "Key Structure"))
  (bind _springarm (`/Game/myContent/blueprints/rtsCameraPawnBP.SpringArm` (`self.cameraPawnRef`)))
  ;[1 1 1] Zoom controls
  (:`Pressed`
    (set `SpringArmComponent.TargetArmLength` (`KismetMathLibrary.FClamp` (- (`SpringArmComponent.TargetArmLength` _springarm) (`self.zoomSpeed`)) (`self.minZoomStop`) (`self.maxZoomStop`)) _springarm)))

(event `InputAction|inpZoomOut`
  (params (Key :type "Key Structure"))
  (bind _springarm (`/Game/myContent/blueprints/rtsCameraPawnBP.SpringArm` (`self.cameraPawnRef`)))
  ;[1 1 1] Zoom controls
  (:`Pressed`
    (set `SpringArmComponent.TargetArmLength` (`KismetMathLibrary.FClamp` (+ (`self.zoomSpeed`) (`SpringArmComponent.TargetArmLength` _springarm)) (`self.minZoomStop`) (`self.maxZoomStop`)) _springarm)))

(event `InputAction|inpViewReset`
  (params (Key :type "Key Structure"))
  ;[1 1 1] Reset View
  (:`Released`
    (`self.K2_SetActorTransform` (`self.cameraPawnRef`) (`self.levelStart`) true false) ; Restore default transform and rotate
  ))

(event `InputAction|inpViewReset`
  (params (Key :type "Key Structure"))
  ;[1 1 1] Reset View
  (:`Released`
    (set `SpringArmComponent.TargetArmLength` (`self.springArmLengthDefault`) (`/Game/myContent/blueprints/rtsCameraPawnBP.SpringArm` (`self.cameraPawnRef`))) ; Go back the the default length we set
  ))

(event `InputAction|inpPanReset`
  (params (Key :type "Key Structure"))
  ;[1 1 1] Reset pitch
  (:`Released`
    (`self.K2_SetActorRotation` (`self.cameraPawnRef`) (.rotation (`self.levelStart`)) false)))

(event `InputAction|inpPan`
  (params (Key :type "Key Structure"))
  (bind _camerapawnref (`self.cameraPawnRef`))
  ;[1 1 1] Pitch and Rotate
  (:`Pressed`
    (set `self.disableCameraMovement` true)
    (goto _label_2 :!via `Open`))
  (:`Released`
    (set `self.disableCameraMovement` false)
    (goto _label_2 :!via `Close`)))

(event `InputAxisKey|MouseX`
  (params (AxisValue :type "Float (single-precision)"))
  (bind _camerapawnref (`self.cameraPawnRef`))
  ;[1 1 1] Pitch and Rotate
  (`/Engine/EditorBlueprintResources/StandardMacros.Gate` true :!label _label_2
    (:`Exit`
      (`self.K2_SetActorRotation` _camerapawnref (`KismetMathLibrary.MakeRotator` (.roll (`self.K2_GetActorRotation` _camerapawnref)) (.pitch (`self.K2_GetActorRotation` _camerapawnref)) (+ (.yaw (`self.K2_GetActorRotation` _camerapawnref)) (* AxisValue (`self.panSpeed`)))) false))))

(event `InputAction|inpPan`
  (params (Key :type "Key Structure"))
  (bind _camerapawnref (`self.cameraPawnRef`))
  ;[1 1 1] Pitch and Rotate
  (:`Pressed`
    (set `self.disableCameraMovement` true)
    (goto _label_3 :!via `Open`))
  (:`Released`
    (set `self.disableCameraMovement` false)
    (goto _label_3 :!via `Close`)))

(event `InputAxisKey|MouseY`
  (params (AxisValue :type "Float (single-precision)"))
  (bind _camerapawnref (`self.cameraPawnRef`))
  ;[1 1 1] Pitch and Rotate
  (`/Engine/EditorBlueprintResources/StandardMacros.Gate` true :!label _label_3
    (:`Exit`
      (`self.K2_SetActorRotation` _camerapawnref (`KismetMathLibrary.MakeRotator` (.roll (`self.K2_GetActorRotation` _camerapawnref)) (`KismetMathLibrary.FClamp` (+ (.pitch (`self.K2_GetActorRotation` _camerapawnref)) (* AxisValue (`self.panSpeed`))) (`self.maxPitch`) (`self.minPitch`)) (.yaw (`self.K2_GetActorRotation` _camerapawnref))) false))))

(event `InputAxisKey|MouseX`
  (params (AxisValue :type "Float (single-precision)"))
  ;[1 1 1] Edge scrolling
  (if (not (`self.disableCameraMovement`))
    (bind (_deltaspeedx _deltaspeedy) (`self.edgeScrolling` :!label _label_4)
      (:`edgeScrollAction`
        (`self.K2_AddActorLocalOffset` (`self.cameraPawnRef`) (`KismetMathLibrary.MakeVector` _deltaspeedx _deltaspeedy) true false)))))

(event `InputAxisKey|MouseY`
  (params (AxisValue :type "Float (single-precision)"))
  ;[1 1 1] Edge scrolling
  (if (not (`self.disableCameraMovement`))
    (goto _label_4 :!via `mouseY`)))

(fn `NewFunction_0`
  (params (self2 :type "Actor Object Reference"))
  (`AddComponent|NODE_AddFloatingPawnMovement-0` :`self` self2))

(fn `UserConstructionScript`)