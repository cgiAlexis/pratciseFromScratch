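; RTS game state Blueprint that runs the in-game clock and calendar from a configured start time and date.
; Each tick, IncrementGameTime advances fractional-hour time at the base game speed and returns a day count.
; SetClock splits time by whole-and-remainder division, while SetCalendar rolls days into months and years; both print on screen and share the GameDate array.
; UpdateGameSpeed stores a multiplier that Tick does not use.
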(event `self.ReceiveBeginPlay`
  (bind _returnvalue (`KismetMathLibrary.Conv_IntToDouble` (`self.hours`)))
  (`|ExecutionSequence`
    (:`then_0`
      (`self.referenceCast`))
    (:`then_1`
      ;[1 1 1] Initialise the start condition time
      (set `self.gameTime` (+ _returnvalue (/ (`KismetMathLibrary.Conv_IntToDouble` (`self.minutes`)) 60.0) (/ _returnvalue 3600.0)))
      (set `self.gameDate` (`|MakeArray` (`self.day`) (`self.month`) (`self.year`))))
    (:`then_2`
      ;[1 1 1] Set starting game speed
      (set `self.baseGameSpeed` (`self.defaultGameSpeed`)))))

(event `self.ReceiveTick`
  (params (DeltaSeconds :type "Float (single-precision)"))
  ;[1 1 1] Progresses game time on game ticks
  (bind (_gametime _daycount) (`/Game/myContent/blueprints/library/rtsFunctionLibraryBP.Increment Game Time` DeltaSeconds (`self.baseGameSpeed`) (`self.gameTime`)))
  (set `self.gameTime` _gametime)
  (set `self.dayCounter` _daycount)
  (`self.setClock`)
  (`self.setCalendar`))

(event `/Game/myContent/blueprints/library/rtsGameTimeIF.updateGameSpeed`
  (params (gameSpeedMultiplier :type "Float (single-precision)"))
  (set `self.gameSpeedMultiplier` gameSpeedMultiplier))

(fn `setCalendar`
  (bind _output_get (set `self.day` (+ (`self.day`) (`self.dayCounter`))))
  (if (> _output_get (`KismetMathLibrary.DaysInMonth` (`self.year`) (`self.month`)))
    ;[1 1 1] Increment month
    (set `self.day` 1)
    (set `self.month` (+ (`self.month`) 1)))
  (if (> (`self.month`) 12)
    ;[1 1 1] Increment year
    (set `self.month` 0)
    (set `self.year` (+ (`self.year`) 1)))
  (bind _output_get_2 (set `self.gameDate` (`|MakeArray` (`self.day`) (`self.month`) (`self.year`))))
  (`KismetSystemLibrary.PrintString` (`KismetStringLibrary.BuildString_Int` (`KismetStringLibrary.BuildString_Int` (`KismetStringLibrary.Conv_IntToString` (`|GetArrayItem` _output_get_2)) " / " (`|GetArrayItem` _output_get_2 1)) " / " (`|GetArrayItem` _output_get_2 2)) true false (struct :`R` 0.141904 :`G` 1.0 :`B` 0.186402 :`A` 1.0) 0.1))

(fn `setClock`
  (bind (_remainder _returnvalue) (`KismetMathLibrary.FMod` (* (`self.gameTime`) 3600.0) 60.0))
  (bind (_remainder_2 _returnvalue_2) (`KismetMathLibrary.FMod` (`KismetMathLibrary.Conv_IntToDouble` _returnvalue) 60.0))
  (set `self.seconds` (`KismetMathLibrary.FFloor` _remainder))
  (set `self.minutes` (`KismetMathLibrary.FFloor` _remainder_2))
  (set `self.hours` (`KismetMathLibrary.FFloor` (`KismetMathLibrary.FMod` (`KismetMathLibrary.Conv_IntToDouble` _returnvalue_2) 24.0)))
  (bind _output_get (set `self.gameDate` (`|MakeArray` (`self.seconds`) (`self.minutes`) (`self.hours`))))
  (`KismetSystemLibrary.PrintString` (`KismetStringLibrary.BuildString_Int` (`KismetStringLibrary.BuildString_Int` (`KismetStringLibrary.Conv_IntToString` (`|GetArrayItem` _output_get 2)) " : " (`|GetArrayItem` _output_get 1) " . ") "" (`|GetArrayItem` _output_get) "s") true false (struct :`G` 0.66 :`B` 1.0 :`A` 1.0) 0.1))

(fn `UserConstructionScript`)